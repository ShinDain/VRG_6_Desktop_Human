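; Actor that acts as a TCP client linking the game to a Python server, exchanging data as strings.
; StartPythonConnection connects to the configured IP and port, with callbacks that track the connection ID and connected state.
; SendDataToPyScript sends strings as bytes, while received bytes are converted, stored and broadcast through IncomingDataFromPython.
; Helpers disconnect and report connection status, and DebuggingEnabled gates on-screen status messages.
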(event Custom|Start%20Python%20Connection
  (bind _connectionid (Class|TcpSocketConnection|Connect (Variables|SocketConnect|GetIp%20Address) (Variables|SocketConnect|GetPort) (|HandleDisconnectfromPython) (|HandleConnectiontoPython) (delegate HandleRecievingDatafromPython)))
  (Variables|SocketConnect|SetConnection%20Id _connectionid))

(fn ConstructionScript)

(fn SendDatatoPyScript
  (params (Data%20as%20String :type String))
  (bind _returnvalue (Class|TcpSocketConnection|SendData (Variables|SocketConnect|GetConnection%20Id) (Class|TcpSocketConnection|ToBytes(String) Data%20as%20String)))
  (if (Variables|Default|GetDebugging%20Enabled)
    (Development|PrintString (Utilities|String|ToString(Text) (Utilities|Text|FormatText "Data Sending was {status}" _returnvalue)) true true "(R=1.000000,G=1.000000,B=0.000000,A=1.000000)" 1e+01 "sdfdv"))
  (return _returnvalue))

(fn DisconnectfromPython
  (Class|TcpSocketConnection|Disconnect (Variables|SocketConnect|GetConnection%20Id))
  (Variables|SocketConnect|SetConnection%20Id 0))

(fn CheckPythonConnected
  (return (Variables|SocketConnect|GetConnected%20To%20Python)))

(event Custom|Disconnected
  (params (ConnectionId :type Integer))
  (Class|TcpSocketConnection|Disconnect (Variables|SocketConnect|GetConnection%20Id))
  (Variables|SocketConnect|SetConnection%20Id 0)
  (Variables|SocketConnect|SetConnected%20To%20Python false)
  (if (Variables|Default|GetDebugging%20Enabled)
    (Development|PrintString (Utilities|String|Append "Warning! Python Server Connection {" (Utilities|String|ToString(Integer) (Variables|SocketConnect|GetConnection%20Id)) "} Has Disconnected!") true true "(R=1.000000,G=1.000000,B=0.000000,A=1.000000)" 1e+01)))

(event Custom|Connected
  (params (ConnectionId :type Integer))
  ;[1 1 1] When Connection Successful To Server
  (Variables|SocketConnect|SetConnected%20To%20Python true)
  (Variables|SocketConnect|SetConnection%20Id ConnectionId)
  (if (Variables|Default|GetDebugging%20Enabled)
    (Development|PrintString (Utilities|String|ToString(Text) (Utilities|Text|FormatText "Connected To Python Successfully;;  IP: {IP},  PORT: {PORT},  CONN_ID: {ID}  " (Variables|SocketConnect|GetIp%20Address) (Variables|SocketConnect|GetPort) (Variables|SocketConnect|GetConnection%20Id))) true true "(R=0.247933,G=1.000000,B=0.000000,A=1.000000)" 2e+01 "dfgds")))

(event Custom|TCP%20Recieved
  (params (ConnectionId :type Integer) (Message :type Array%20of%20Bytes))
  ;[1 1 1] On Recieved Data From TCP Server
  (bind _returnvalue (Class|PythonFunctionLibrary|ConvertBytestoString Message))
  (Variables|Default|SetRecieved%20Data _returnvalue)
  (if (Variables|Default|GetDebugging%20Enabled)
    (Development|PrintString (Utilities|String|ToString(Text) (Utilities|Text|FormatText "Incoming Data Recieved from;;  IP: {ip},  PORT: {port},  CONN_ID:  {con_id}" (Variables|SocketConnect|GetIp%20Address) (Variables|SocketConnect|GetPort) (Variables|SocketConnect|GetConnection%20Id))) true true "(R=0.000000,G=1.000000,B=0.000000,A=1.000000)" 1e+01 "dsfvss"))
  (Default|CallIncomingDatafromPython (Variables|Default|GetRecieved%20Data)))