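; BP_TCP_Test is a test Blueprint that exercises two-way data exchange with a Python script through BP_Python_Runtime_Connect.
; On BeginPlay it finds that actor, binds a handler to its incoming-data event and starts the connection.
; A looping half-second timer steps through a list of strings with a wrapping index and sends each to the script, while replies are stored and printed.
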(event Custom|On%20Python%20Reply
  (params (Data :type String))
  (bind _output_get (Variables|Default|SetIn%20Data Data))
  (Development|PrintString _output_get))

(event Custom|Send%20Python%20Data%20to%20Script
  (bind _result (Math|Integer|IncrementInt (Variables|Default|GetIndex))
    (:%20%20
      (if (> _result (Utilities|Array|Length (Variables|Default|GetList%20Of%20%20Data%20Strings)))
        (Variables|Default|SetIndex 0))
      (Variables|Default|SetOut%20Data (Utilities|Array|Get(acopy) (Variables|Default|GetList%20Of%20%20Data%20Strings) (Variables|Default|GetIndex)))
      (Default|SendDatatoPyScript (Variables|Default|GetPython%20Communication%20Ref) (Variables|Default|GetOut%20Data)))))

(event EventBeginPlay
  (bind _returnvalue (Actor|GetActorOfClass "/Game/Blueprints/Python_TCP_Connect/BP_Python_Runtime_Connect.BP_Python_Runtime_Connect_C"))
  (bind _output_get (Variables|Default|SetPython%20Communication%20Ref _returnvalue))
  (EventDispatchers|BindEventtoIncomingDatafromPython _output_get (delegate Custom|On%20Python%20Reply))
  (Default|StartPythonConnection _output_get)
  (Utilities|Time|SetTimerbyEvent (delegate Custom|Send%20Python%20Data%20to%20Script) 0.5 true))

(fn ConstructionScript)